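; BP_OmniMovePawn is a player pawn with omni-movement abilities (jump, crouch-slide, dash, grapple) and weapon fire.
; On BeginPlay it adds the IMC_Player mapping context and creates the WB_CharacterCD widget on screen.
; Enhanced Input events forward to the movement and combat components, which hold the actual logic, with dash also receiving the current move input.
; The movement component's grapple start and stop events toggle the Grapple component's visibility.
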(event `self.ReceiveBeginPlay`
  (bind _asplayer_controller (cast `PlayerController` (`self.GetController`)))
  (bind _returnvalue (pcsubsystem `EnhancedInputLocalPlayerSubsystem` _asplayer_controller))
  (`/Engine/EditorBlueprintResources/StandardMacros.IsValid` _returnvalue
    (:`Is Valid`
      (`EnhancedInputSubsystemInterface.AddMappingContext` _returnvalue "/Game/Input/Contexts/IMC_Player.IMC_Player" 0 (struct))
      (bind _returnvalue_2 (`|CreateWidget` "/Game/Widget/WB_CharacterCD.WB_CharacterCD_C" (`GameplayStatics.GetPlayerController` 0)))
      (`UserWidget.AddToViewport` _returnvalue_2 0))))

(event `EnhancedInput|/Game/Input/Actions/IA_Moves`
  (params (ActionValue :type "Vector2D Structure") (ElapsedSeconds :type "Float (double-precision)") (TriggeredSeconds :type "Float (double-precision)") (InputAction :type "InputAction Object Reference" :default "/Game/Input/Actions/IA_Moves.IA_Moves"))
  (:`Triggered`
    (`AC_BaseMovement.Move` (`self.AC_BaseMovement`) ActionValue)))

(event `EnhancedInput|/Game/Input/Actions/IA_Look`
  (params (ActionValue :type "Vector2D Structure") (ElapsedSeconds :type "Float (double-precision)") (TriggeredSeconds :type "Float (double-precision)") (InputAction :type "InputAction Object Reference" :default "/Game/Input/Actions/IA_Look.IA_Look"))
  (:`Triggered`
    (`AC_BaseMovement.Look` (`self.AC_BaseMovement`) ActionValue)))

(event `EnhancedInput|/Game/Input/Actions/IA_Jump`
  (params (ActionValue :type Boolean) (ElapsedSeconds :type "Float (double-precision)") (TriggeredSeconds :type "Float (double-precision)") (InputAction :type "InputAction Object Reference" :default "/Game/Input/Actions/IA_Jump.IA_Jump"))
  (:`Started`
    (`AC_BaseMovement.TriggerJump` (`self.AC_BaseMovement`))))

(event `EnhancedInput|/Game/Input/Actions/IA_Crouch`
  (params (ActionValue :type Boolean) (ElapsedSeconds :type "Float (double-precision)") (TriggeredSeconds :type "Float (double-precision)") (InputAction :type "InputAction Object Reference" :default "/Game/Input/Actions/IA_Crouch.IA_Crouch"))
  (bind _ac_basemovement (`self.AC_BaseMovement`))
  (:`Triggered`
    (`AC_BaseMovement.StartCrouchSlide` _ac_basemovement))
  (:`Completed`
    (`AC_BaseMovement.StopCrouchSlide` _ac_basemovement)))

(event `EnhancedInput|/Game/Input/Actions/IA_Dash`
  (params (ActionValue :type Boolean) (ElapsedSeconds :type "Float (double-precision)") (TriggeredSeconds :type "Float (double-precision)") (InputAction :type "InputAction Object Reference" :default "/Game/Input/Actions/IA_Dash.IA_Dash"))
  (:`Started`
    (`AC_BaseMovement.TriggerDash` (`self.AC_BaseMovement`) (`|GetInputActionValue`))))

(event `EnhancedInput|/Game/Input/Actions/IA_Grappling`
  (params (ActionValue :type Boolean) (ElapsedSeconds :type "Float (double-precision)") (TriggeredSeconds :type "Float (double-precision)") (InputAction :type "InputAction Object Reference" :default "/Game/Input/Actions/IA_Grappling.IA_Grappling"))
  (bind _ac_basemovement (`self.AC_BaseMovement`))
  (:`Started`
    (`AC_BaseMovement.StartGrapple` _ac_basemovement))
  (:`Canceled`
    (`AC_BaseMovement.StopGrapple` _ac_basemovement :!label _label))
  (:`Completed`
    (goto _label)))

(event `self.AC_BaseMovement.OnGrappleStarted`
  (`SceneComponent.SetHiddenInGame` (`self.Grapple`) false false))

(event `self.AC_BaseMovement.OnGrappleStopped`
  (`SceneComponent.SetHiddenInGame` (`self.Grapple`) true false))

(event `EnhancedInput|/Game/Input/Actions/IA_Fire`
  (params (ActionValue :type Boolean) (ElapsedSeconds :type "Float (double-precision)") (TriggeredSeconds :type "Float (double-precision)") (InputAction :type "InputAction Object Reference" :default "/Game/Input/Actions/IA_Fire.IA_Fire"))
  (:`Triggered`
    (`AC_Combat.StartFire` (`self.AC_Combat`)))
  (:`Canceled`
    (`AC_Combat.StopFire` (`self.AC_Combat`) :!label _label_2))
  (:`Completed`
    (goto _label_2)))

(fn `UserConstructionScript`)