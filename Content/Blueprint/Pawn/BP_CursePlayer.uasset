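; Player character for a curse-driven game, with movement, jump, camera zoom, a grappling hook and a pause menu.
; A looping timer samples height changes and raises the curse stored in BP_PS_PlayerData on ascent or lowers it on descent.
; A dynamic post-process material exposes curse intensity for visual feedback.
; The grapple line-traces from the camera, then switches to flying and pulls toward the hit point with a visible cable.
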(event `self.ReceiveBeginPlay`
  ; Player's BeginPlay
  (bind _asplayer_controller (cast `PlayerController` (`self.GetController`)))
  (bind _returnvalue (pcsubsystem `EnhancedInputLocalPlayerSubsystem` _asplayer_controller))
  (`/Engine/EditorBlueprintResources/StandardMacros.IsValid` _returnvalue
    (:`Is Valid`
      (`EnhancedInputSubsystemInterface.AddMappingContext` _returnvalue "/Game/Input/Contexts/IMC_Player.IMC_Player" 0 (struct))
      (bind _asbp_ps_player_data (cast `/Game/Blueprint/BP_PS_PlayerData` (`GameplayStatics.GetPlayerState` 0)))
      (set `self.CachedPlayerState` _asbp_ps_player_data)
      (set `self.LastHeightPos` (.z (`self.K2_GetActorLocation`)))
      (`KismetSystemLibrary.K2_SetTimer` null "CheckAltitude" 0.2 true)
      (bind _returnvalue_2 (`KismetMaterialLibrary.CreateDynamicMaterialInstance` "/Game/Post-Process/M_CursePostProcess_InstTest.M_CursePostProcess_InstTest"))
      (bind _output_get (set `self.PostProcessMatInst` _returnvalue_2))
      (`PostProcessComponent.AddOrUpdateBlendable` (`self.CursePostProcess`) _output_get 1.0)
      (add `/Game/Blueprint/BP_PS_PlayerData.OnCursedChanged` (`self.CachedPlayerState`) (`|CreateDelegate` :!event `UpdateCursePostProcessMat`)))))

(event `EnhancedInput|/Game/Input/Actions/IA_Jump`
  (params (ActionValue :type Boolean) (ElapsedSeconds :type "Float (double-precision)") (TriggeredSeconds :type "Float (double-precision)") (InputAction :type "InputAction Object Reference" :default "/Game/Input/Actions/IA_Jump.IA_Jump"))
  ; Player's Jump
  (:`Triggered`
    (`self.Jump`))
  (:`Completed`
    (`self.StopJumping`)))

(event `EnhancedInput|/Game/Input/Actions/IA_CamZoom`
  (params (ActionValue :type "Vector2D Structure") (ElapsedSeconds :type "Float (double-precision)") (TriggeredSeconds :type "Float (double-precision)") (InputAction :type "InputAction Object Reference" :default "/Game/Input/Actions/IA_CamZoom.IA_CamZoom"))
  (:`Triggered`
    (set `SpringArmComponent.TargetArmLength` (`KismetMathLibrary.Conv_IntToDouble` (`KismetMathLibrary.Clamp` (`KismetMathLibrary.FTrunc` (+ (* ActionValue_X -25.0) (`SpringArmComponent.TargetArmLength` (`self.SpringArm`)))) 300 1200)) (`self.SpringArm`))))

(event `EnhancedInput|/Game/Input/Actions/IA_Look`
  (params (ActionValue :type "Vector2D Structure") (ElapsedSeconds :type "Float (double-precision)") (TriggeredSeconds :type "Float (double-precision)") (InputAction :type "InputAction Object Reference" :default "/Game/Input/Actions/IA_Look.IA_Look"))
  ; Mouse Movement
  (:`Triggered`
    (`self.AddControllerYawInput` ActionValue_X)
    (`self.AddControllerPitchInput` ActionValue_Y)))

(event `EnhancedInput|/Game/Input/Actions/IA_Moves`
  (params (ActionValue :type "Vector2D Structure") (ElapsedSeconds :type "Float (double-precision)") (TriggeredSeconds :type "Float (double-precision)") (InputAction :type "InputAction Object Reference" :default "/Game/Input/Actions/IA_Moves.IA_Moves"))
  (bind (_returnvalue_roll _returnvalue_pitch _returnvalue_yaw) (`KismetMathLibrary.BreakRotator` (`self.GetControlRotation`)))
  (bind (_returnvalue_roll_2 _returnvalue_pitch_2 _returnvalue_yaw_2) (`KismetMathLibrary.BreakRotator` (`self.GetControlRotation`)))
  ; Character Movement
  (:`Triggered`
    (`self.AddMovementInput` (`KismetMathLibrary.GetRightVector` (`KismetMathLibrary.MakeRotator` _returnvalue_roll 0.0 _returnvalue_yaw)) ActionValue_X)
    (`self.AddMovementInput` (`KismetMathLibrary.GetForwardVector` (`KismetMathLibrary.MakeRotator` 0.0 0.0 _returnvalue_yaw_2)) ActionValue_Y)))

(event `self.ReceiveTick`
  (params (DeltaSeconds :type "Float (single-precision)"))
  ; GrapplingHook
  (`/Game/Blueprint/BP_PS_PlayerData.GetCurse` (`self.CachedPlayerState`))
  (if (`self.IsGrappled`)
    (set `CableComponent.EndLocation` (`KismetMathLibrary.InverseTransformLocation` (`self.GetTransform`) (`self.GrabbedPoint`)) (`self.Cable`))
    (`CharacterMovementComponent.AddForce` (`self.CharacterMovement`) (* (`KismetMathLibrary.Normal` (+ (`KismetMathLibrary.GetDirectionUnitVector` (`self.K2_GetActorLocation`) (`self.GrabbedPoint`)) (* (* (`self.GetActorRightVector`) (`.Y` (`KismetMathLibrary.BreakVector2D` (stale `EnhancedInput|/Game/Input/Actions/IA_Moves` ActionValue)))) 0.7))) 500000.0))))

(event `EnhancedInput|/Game/Input/Actions/IA_Grappling`
  (params (ActionValue :type Boolean) (ElapsedSeconds :type "Float (double-precision)") (TriggeredSeconds :type "Float (double-precision)") (InputAction :type "InputAction Object Reference" :default "/Game/Input/Actions/IA_Grappling.IA_Grappling"))
  (bind _camera (`self.Camera`))
  (bind _returnvalue (`SceneComponent.K2_GetComponentLocation` _camera))
  ; GrapplingHook
  (:`Started`
    (bind (_outhit _returnvalue_2) (`KismetSystemLibrary.LineTraceSingle` :`Start` _returnvalue :`End` (+ _returnvalue (* (`KismetMathLibrary.GetForwardVector` (`SceneComponent.K2_GetComponentRotation` _camera)) 10000.0)) :`TraceChannel` "TraceTypeQuery1" :`bTraceComplex` true :`DrawDebugType` "ForOneFrame"))
    (if _returnvalue_2
      (set `self.GrabbedPoint` (`.ImpactPoint` (`GameplayStatics.BreakHitResult` _outhit)))
      (set `self.IsGrappled` true)
      (`CharacterMovementComponent.SetMovementMode` (`self.CharacterMovement`) "MOVE_Flying" 0)
      (`SceneComponent.SetVisibility` (`self.Cable`) true false)))
  (:`Completed`
    (set `self.IsGrappled` false)
    (`CharacterMovementComponent.SetMovementMode` (`self.CharacterMovement`) "MOVE_Falling" 0)
    (`SceneComponent.SetVisibility` (`self.Cable`) false false)))

(event `EnhancedInput|/Game/Input/Actions/IA_OpenMenu`
  (params (ActionValue :type Boolean) (ElapsedSeconds :type "Float (double-precision)") (TriggeredSeconds :type "Float (double-precision)") (InputAction :type "InputAction Object Reference" :default "/Game/Input/Actions/IA_OpenMenu.IA_OpenMenu"))
  (bind _returnvalue (`GameplayStatics.GetPlayerController` 0))
  (bind _pausemenu (`self.PauseMenu`))
  ; UI
  (:`Started`
    (if (not (`self.isPaused?`))
      (set `self.isPaused?` true)
      (bind _returnvalue_2 (`|GenericCreateObject` _returnvalue "/Game/UI/SystemUI/WBP_PauseMenu.WBP_PauseMenu_C"))
      (bind _output_get (set `self.PauseMenu` _returnvalue_2))
      (`UserWidget.AddToViewport` _output_get 0)
      (`WidgetBlueprintLibrary.SetInputMode_UIOnlyEx` _returnvalue _pausemenu)
      (set `PlayerController.bShowMouseCursor` true _returnvalue)
      (`GameplayStatics.SetGamePaused` true)
      (else
        (set `self.isPaused?` false)
        (`Widget.RemoveFromParent` _pausemenu)
        (`WidgetBlueprintLibrary.SetInputMode_GameOnly` _returnvalue)
        (set `PlayerController.bShowMouseCursor` false _returnvalue)
        (`GameplayStatics.SetGamePaused` false)))))

(fn `CheckAltitude`
  (locals (CurrentZ :type "Float (double-precision)") (DeltaZ :type "Float (double-precision)"))
  (bind _cachedplayerstate (`self.CachedPlayerState`))
  ; Getting Last&New Position to see if we got through the required Threshold to Update the Curse
  (bind _output_get (set `local.CurrentZ` (.z (`self.K2_GetActorLocation`))))
  (bind _output_get_2 (set `local.DeltaZ` (- _output_get (`self.LastHeightPos`))))
  (if (>= (`KismetMathLibrary.Abs` _output_get_2) (`self.ZThreshold`))
    (if (> (`local.DeltaZ`) 0.0)
      ; Go Up -> Curse go Up
      (`/Game/Blueprint/BP_PS_PlayerData.ModifyCurse` _cachedplayerstate (* (* (`self.CurseBaseAmount`) (`self.CurseMultiplierUp`)) (/ (`local.DeltaZ`) 100.0)))
      (else
        ; Go Down -> Curse Go Down
        (`/Game/Blueprint/BP_PS_PlayerData.ModifyCurse` _cachedplayerstate (* (* (* (`self.CurseBaseAmount`) (`self.CurseMultiplierDown`)) (/ (`KismetMathLibrary.Abs` (`local.DeltaZ`)) 100.0)) -1.0))))
    (set `self.LastHeightPos` (`local.CurrentZ`))
    (else
      (set `self.LastHeightPos` (`local.CurrentZ`)))))

(fn `UpdateCursePostProcessMat`
  (params (NewValue :type "Float (double-precision)") (Ratio :type "Float (double-precision)"))
  (`MaterialInstanceDynamic.SetScalarParameterValue` (`self.PostProcessMatInst`) "CurseIntensity" NewValue))

(fn `UserConstructionScript`)