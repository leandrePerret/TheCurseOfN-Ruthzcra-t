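; Character grappling hook: holding the left mouse button grapples to a line-trace impact point and pulls the character toward it.
; Press stores the point, switches movement to Flying and shows the Cable; release returns to Falling and hides it.
; While grappled, Tick pins the cable end to the point in local space and adds a constant-magnitude force toward it, biased along the actor's right vector.
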(event `Key|LeftMouseButton`
  (params (Key :type "Key Structure"))
  ; Grappin
  (:`Pressed`
    (bind _outhit (`KismetSystemLibrary.LineTraceSingle` :`End` (+ (0.0 0.0 0.0) (* (0.0 0.0 0.0) 3000.0)) :`TraceChannel` "TraceTypeQuery1" :`DrawDebugType` "ForOneFrame"))
    (if true
      (set `self.Grabbed Point` (`.ImpactPoint` (`GameplayStatics.BreakHitResult` _outhit)))
      (set `self.IsGrappled` true)
      (`CharacterMovementComponent.SetMovementMode` (`self.CharacterMovement`) "MOVE_Flying" 0)
      (`SceneComponent.SetVisibility` (`self.Cable`) true false)))
  (:`Released`
    (set `self.IsGrappled` false)
    (`CharacterMovementComponent.SetMovementMode` (`self.CharacterMovement`) "MOVE_Falling" 0)
    (`SceneComponent.SetVisibility` (`self.Cable`) false false)))

(event `self.ReceiveTick`
  (params (DeltaSeconds :type "Float (single-precision)"))
  (if (`self.IsGrappled`)
    (set `CableComponent.EndLocation` (`KismetMathLibrary.InverseTransformLocation` (`self.GetTransform`) (`self.Grabbed Point`)) (`self.Cable`))
    (`CharacterMovementComponent.AddForce` (`self.CharacterMovement`) (* (`KismetMathLibrary.Normal` (+ (`KismetMathLibrary.GetDirectionUnitVector` (`self.K2_GetActorLocation`) (`self.Grabbed Point`)) (* (* (`self.GetActorRightVector`) 0.0) 0.7))) 250000.0))))

(fn `UserConstructionScript`)