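; Barred door actor that opens when all of its required levers are activated.
; Levers toggle themselves in an activated list; adding one rechecks the combination, and removing one closes an open door.
; A timeline slides the bars from their starting location by an offset and reverses to close, adding a child actor component each way.
; Ordered combinations are only a placeholder print.
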(event `self.ReceiveBeginPlay`
  (set `self.ClosedLocation` (`SceneComponent.K2_GetComponentLocation` (`self.SM_Bars`))))

(event `OpenDoor`
  (set `self.bIsOpen` true)
  (`AddComponent|NODE_AddChildActorComponent-0`)
  (bind (_direction _doortrack) (`Timeline|DoorTimeline` :!label _label)
    (:`Update`
      (`SceneComponent.K2_SetWorldLocation` (`self.SM_Bars`) (`KismetMathLibrary.VLerp` (`self.ClosedLocation`) (+ (`self.ClosedLocation`) (`self.OpeningOffset`)) _doortrack) false false))))

(event `CloseDoor`
  (set `self.bIsOpen` false)
  (`AddComponent|NODE_AddChildActorComponent-1`)
  (goto _label :!via `Reverse`))

(fn `AddLeverToArray`
  (params (LeverActor :type "Actor Object Reference"))
  (bind _activatedlevers (`self.ActivatedLevers`))
  (`KismetSystemLibrary.PrintString` "Add LEVER")
  (if (`KismetArrayLibrary.Array_Contains` (`self.ActivatedLevers`) LeverActor)
    (`self.RemoveLeverFromArray` LeverActor)
    (return)
    (else
      (`KismetArrayLibrary.Array_Add` _activatedlevers LeverActor)
      (`KismetSystemLibrary.PrintString` (`KismetStringLibrary.Conv_IntToString` (`KismetArrayLibrary.Array_Length` _activatedlevers)))
      (`self.CheckCombination`))))

(fn `CheckCombination`
  (locals (bIsLoopBroken :type Boolean))
  (if (`self.bRequiresOrder`)
    (`KismetSystemLibrary.PrintString` "I didn't do the Order Logic Yet")
    (else
      (set `local.bIsLoopBroken` true)
      (for _array_element (`self.RequiredLevers`)
        (if (not (`KismetArrayLibrary.Array_Contains` (`self.ActivatedLevers`) _array_element))
          (set `local.bIsLoopBroken` false)))
      (if (`local.bIsLoopBroken`)
        (`self.OpenDoor`)))))

(fn `RemoveLeverFromArray`
  (params (LeverActor :type "Actor Object Reference"))
  (`KismetSystemLibrary.PrintString` "removing It")
  (if (`KismetArrayLibrary.Array_Contains` (`self.ActivatedLevers`) LeverActor)
    (bind _returnvalue (`KismetArrayLibrary.Array_RemoveItem` (`self.ActivatedLevers`) LeverActor))
    (if _returnvalue
      (if (`self.bIsOpen`)
        (`self.CloseDoor`)
        (else
          (return)))
      (else
        (return)))
    (else
      (return))))

(fn `UserConstructionScript`)