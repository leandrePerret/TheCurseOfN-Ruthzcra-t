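; Player data Blueprint, likely a PlayerState, that tracks a player's curse meter with getter, reset and modify functions.
; ModifyCurse clamps the value, broadcasts it with its ratio through OnCursedChanged, and restarts a decay delay timer on positive amounts.
; After the delay, a looping timer drains the curse in small steps, broadcasting each change until it reaches the minimum.
; ResetCurse zeroes the value without broadcasting or touching the timer.
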(fn `GetCurse`
  (returns (CurseValue :type "Float (double-precision)"))
  (return (`self.CurseValue`)))

(fn `ModifyCurse`
  (params (Amount :type "Float (double-precision)"))
  (bind _cursemax (`self.CurseMax`))
  (bind _output_get (set `self.CurseValue` (`KismetMathLibrary.FClamp` (+ (`self.CurseValue`) Amount) (`self.CurseMin`) _cursemax)))
  (`self.OnCursedChanged` _output_get (/ _output_get _cursemax))
  (if (> Amount 0.0)
    (`KismetSystemLibrary.K2_ClearAndInvalidateTimerHandle` (`self.DecayTimerHandle`))
    (bind _returnvalue (`KismetSystemLibrary.K2_SetTimer` null "StartDecay" (`self.CurseDecayDelay`)))
    (set `self.DecayTimerHandle` _returnvalue)))

(fn `ResetCurse`
  (set `self.CurseValue` 0.0))

(fn `StartDecay`
  (set `self.bDecayActive` true)
  (bind _returnvalue (`KismetSystemLibrary.K2_SetTimer` null "TickDecay" 0.1 true))
  (set `self.DecayTimerHandle` _returnvalue))

(fn `TickDecay`
  (if (<= (`self.CurseValue`) (`self.CurseMin`))
    (`KismetSystemLibrary.K2_ClearAndInvalidateTimerHandle` (`self.DecayTimerHandle`))
    (set `self.bDecayActive` false)
    (else
      (bind _output_get (set `self.CurseValue` (`KismetMathLibrary.FClamp` (- (`self.CurseValue`) (* (`self.CurseDecayRate`) 0.1)) (`self.CurseMin`) (`self.CurseMax`))))
      (`self.OnCursedChanged` _output_get (/ (`self.CurseValue`) (`self.CurseMax`))))))

(fn `UserConstructionScript`)