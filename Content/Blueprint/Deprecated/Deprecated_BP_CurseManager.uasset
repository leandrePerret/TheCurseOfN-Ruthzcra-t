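; Deprecated curse manager, apparently meant to drive the player's curse value from changes in height.
; On BeginPlay it sets ascend and descend multipliers, caches the player and player state, and starts a looping timer calling CurseHeightCalculation on BP_PS_PlayerData.
; Its own CurseHeightCalculation is empty.
; Disconnected leftover nodes scale height deltas by separate climb and descent multipliers, without writing the curse value.
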(event `self.ReceiveBeginPlay`
  (bind _returnvalue (`GameplayStatics.GetPlayerCharacter` 0))
  (set `self.CurseAscendMultiplicator` 1.3)
  (set `self.CurseDescendMultiplicator` 1.1)
  (set `self.PreviousHeight` (.z (`self.K2_GetActorLocation` _returnvalue)))
  (`/Engine/EditorBlueprintResources/StandardMacros.IsValid` _returnvalue
    (:`Is Valid`
      (`KismetSystemLibrary.PrintString` "VALIIIIIIIIDE")
      (bind _asbp_curse_player (cast `/Game/Blueprint/BP_CursePlayer` _returnvalue))
      (set `self.BP_CursePlayerRef` _asbp_curse_player)
      (bind _asbp_ps_player_data (cast `/Game/Blueprint/BP_PS_PlayerData` (`Controller.PlayerState` (`GameplayStatics.GetPlayerController` 0))))
      (set `self.CachedPlayerState` _asbp_ps_player_data)
      (`KismetSystemLibrary.K2_SetTimer` _asbp_ps_player_data "CurseHeightCalculation" 0.033 true))
    (:`Is Not Valid`
      (`KismetSystemLibrary.PrintString` "PAS VALIDE"))))

(event `self.ReceiveTick`
  (params (DeltaSeconds :type "Float (single-precision)")))

(fn `CurseHeightCalculation`)

(fn `UserConstructionScript`)