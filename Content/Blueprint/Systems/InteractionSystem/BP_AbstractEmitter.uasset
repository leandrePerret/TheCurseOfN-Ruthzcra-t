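; Abstract base actor for interactable emitters in the interaction system, which signal a set of receiver actors.
; Interact calls EmittMessage, which loops over ReceiverActors and sends ActiveState and itself to each one implementing BPI_Receiver.
; Reset overwrites ActiveState, while getters expose hold duration, interaction type and activation state.
; GetWidgetOffsetComp returns nothing here.
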(event `/Game/Blueprint/Systems/InteractionSystem/BPI_Interactable.Interact`
  (params (InteractActorRef :type "Actor Object Reference"))
  (`self.EmittMessage`))

(fn `EmittMessage`
  (for _array_element (`self.ReceiverActors`)
    (if (`KismetSystemLibrary.DoesImplementInterface` _array_element "/Game/Blueprint/Systems/InteractionSystem/BPI_Receiver.BPI_Receiver_C")
      (message `/Game/Blueprint/Systems/InteractionSystem/BPI_Receiver.ReceiveMessage` _array_element (`self.ActiveState`) self))))

(fn `GetHoldDuration`
  (returns (duration :type "Float (double-precision)"))
  (return (`self.HoldDuration`)))

(fn `GetInteractionType`
  (returns (Type :type "/Game/Blueprint/Systems/InteractionSystem/E_InteractionType Enum"))
  (return (`self.InteractionType`)))

(fn `GetIsActivated`
  (returns (IsActivated :type Boolean))
  (return (`self.IsActivated`)))

(fn `GetWidgetOffsetComp`
  (returns (OffsetComp :type "SceneComponent Object Reference"))
  (return null))

(fn `Reset`
  (params (NewActive :type Boolean))
  (set `self.ActiveState` NewActive))

(fn `UserConstructionScript`)