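; Interactable lever that toggles on each instant use, adding or removing itself from a target door's lever array and driving an optional trap.
; A timeline tilts the lever mesh in pitch, playing forward or in reverse.
; Each update of that timeline plays or reverses a second timeline, which slides the trap actor between its starting location and an offset.
; Debug prints remain throughout, and the door reference is used without a validity check.
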(event `self.ReceiveBeginPlay`
  (bind _targettrap (`self.TargetTrap`))
  (set `self.BaseRotation` (`SceneComponent.RelativeRotation` (`self.Cube1`)))
  (`/Engine/EditorBlueprintResources/StandardMacros.IsValid` _targettrap
    (:`Is Valid`
      (set `self.TrapLocation` (`self.K2_GetActorLocation` _targettrap)))))

(event `self.Interact`
  (params (InteractActorRef :type "Actor Object Reference"))
  (bind _targettrap (`self.TargetTrap`))
  (bind _pitch (.pitch (`self.BaseRotation`)))
  (if (`self.bActivated`)
    (`KismetSystemLibrary.PrintString` "Flop B")
    (set `self.bActivated` false)
    (`/Game/Blueprint/BP_BarsDoor.RemoveLeverFromArray` (`self.TargetDoor`) self)
    (bind (_direction _levertrack) (`Timeline|Timeline` :!via `Reverse` :!label _label)
      (:`Update`
        (`SceneComponent.K2_SetRelativeRotation` (`self.Cube1`) (`KismetMathLibrary.MakeRotator` 0.0 (`KismetMathLibrary.Lerp` _pitch (+ _pitch (.pitch (`self.ActivatedOffset`))) _levertrack)) false false)
        (`KismetSystemLibrary.PrintString` "Got after Rotation")
        (`/Engine/EditorBlueprintResources/StandardMacros.IsValid` (`self.TargetTrap`)
          (:`Is Valid`
            (`KismetSystemLibrary.PrintString` "Got through Valid")
            (if (`self.bActivated`)
              (bind (_direction_2 _traptrack) (`Timeline|Timeline_0` :!label _label_2)
                (:`Update`
                  (`KismetSystemLibrary.PrintString` (`KismetStringLibrary.Conv_VectorToString` (`self.K2_GetActorLocation` _targettrap)))
                  (`self.K2_SetActorLocation` _targettrap (`KismetMathLibrary.VLerp` (`self.TrapLocation`) (+ (`self.TrapLocation`) (`self.TrapMovingOffset`)) _traptrack) false false)))
              (else
                (goto _label_2 :!via `Reverse`)))))))
    (else
      (`KismetSystemLibrary.PrintString` "Flip A")
      (set `self.bActivated` true)
      (`/Game/Blueprint/BP_BarsDoor.AddLeverToArray` (`self.TargetDoor`) self)
      (goto _label))))

(fn `GetCanInteract`
  (returns (canInteract :type Boolean))
  (return true))

(fn `GetHoldDuration`
  (returns (duration :type "Float (double-precision)"))
  (return 0.0))

(fn `GetInteractionType`
  (returns (Type :type "/Game/Blueprint/Systems/InteractionSystem/E_InteractionType Enum"))
  (return "NewEnumerator0"))

(fn `GetWidgetOffsetComp`
  (returns (OffsetComp :type "SceneComponent Object Reference"))
  (return null))

(fn `UserConstructionScript`)